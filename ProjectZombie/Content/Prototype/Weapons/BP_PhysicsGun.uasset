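; Physics gun weapon that lets its owner grab, carry, drop and launch physics-simulated objects.
; Primary fire line-traces from the first-person camera and grabs a simulating component with a PhysicsHandle, whose target follows PhysObjLocation every tick; releasing fire drops it.
; Alt fire launches the component from that grab trace along camera forward with a mass-independent impulse, then releases it.
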(event `self.ReceiveTick`
  (params (DeltaSeconds :type "Float (single-precision)"))
  ;[1 1 1] Update physics object location every frame
  (`parent.ReceiveTick` DeltaSeconds)
  (`PhysicsHandleComponent.SetTargetLocation` (`self.PhysicsHandle`) (`SceneComponent.K2_GetComponentLocation` (`self.PhysObjLocation`))))

(event `self.StartFire`
  (bind _firstpersoncameracomponent (`/Game/Prototype/Characters/BP_PlayerCharacter.FirstPersonCameraComponent` (`self.WeaponOwner`)))
  (bind _returnvalue (`SceneComponent.K2_GetComponentLocation` _firstpersoncameracomponent))
  ;[1 1 1] Grap physics object from the world
  (if (not (`self.HasPhysicsObject`))
    (bind (_outhit _returnvalue_2) (`KismetSystemLibrary.LineTraceSingle` :`Start` _returnvalue :`End` (+ _returnvalue (* (`SceneComponent.GetForwardVector` _firstpersoncameracomponent) (`self.GrapDistance`))) :`TraceChannel` "TraceTypeQuery1" :`bTraceComplex` true :`DrawDebugType` "ForDuration"))
    (if _returnvalue_2
      (bind (_bblockinghit _binitialoverlap _time _distance _location _impactpoint _normal _impactnormal _physmat _hitactor _hitcomponent) (`GameplayStatics.BreakHitResult` _outhit))
      (if (`SceneComponent.IsSimulatingPhysics` _hitcomponent "None")
        (`PhysicsHandleComponent.GrabComponentAtLocationWithRotation` :`self` (`self.PhysicsHandle`) :`Component` _hitcomponent :`Location` (`SceneComponent.K2_GetComponentLocation` _hitcomponent))
        (set `self.HasPhysicsObject` true)))))

(event `self.StopFire`
  ;[1 1 1] Drop physics object
  (if (`self.HasPhysicsObject`)
    (`self.DropObject`)))

(event `self.StartAltFire`
  ;[1 1 1] Launch physics objects
  (if (`self.HasPhysicsObject`)
    (`self.LaunchObject` (`.HitComponent` (`GameplayStatics.BreakHitResult` (stale `self.StartFire` _outhit))))
    (`self.DropObject`)))

(fn `DropObject`
  (`PhysicsHandleComponent.ReleaseComponent` (`self.PhysicsHandle`))
  (set `self.HasPhysicsObject` false))

(fn `GetHitResult`
  (returns (OutHit :type "HitResult Structure"))
  (bind _firstpersoncameracomponent (`/Game/Prototype/Characters/BP_PlayerCharacter.FirstPersonCameraComponent` (`self.WeaponOwner`)))
  (bind _returnvalue (`SceneComponent.K2_GetComponentLocation` _firstpersoncameracomponent))
  (bind (_outhit _returnvalue_2) (`KismetSystemLibrary.LineTraceSingle` :`Start` _returnvalue :`End` (+ _returnvalue (* (`SceneComponent.GetForwardVector` _firstpersoncameracomponent) (`self.GrapDistance`))) :`TraceChannel` "TraceTypeQuery1" :`bTraceComplex` true :`DrawDebugType` "ForDuration"))
  (if _returnvalue_2
    (return _outhit)))

(fn `GetIsHeld`
  (returns (IsHeld :type Boolean))
  (return (`self.HasPhysicsObject`)))

(fn `LaunchObject`
  (params (Primitive :type "PrimitiveComponent Object Reference"))
  (if (`self.HasPhysicsObject`)
    (`PrimitiveComponent.AddImpulse` Primitive (* (`SceneComponent.GetForwardVector` (`/Game/Prototype/Characters/BP_PlayerCharacter.FirstPersonCameraComponent` (`self.WeaponOwner`))) (`self.LaunchImpulse`)) "None" true)))

(fn `UserConstructionScript`
  (`parent.UserConstructionScript`))