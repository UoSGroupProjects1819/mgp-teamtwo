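; Base weapon Blueprint for a first-person prototype, handling ownership and attachment to the wielder.
; GiveTo and Remove set or clear the weapon owner, actor owner and instigator.
; AttachToOwner, a separate function, snaps the weapon mesh to a hands socket on the owner's first-person mesh.
; Primary and alt fire events, projectile and instant-hit functions, and DetachFromOwner are empty stubs.
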(event `StartFire`)

(event `StartAltFire`)

(event `StopFire`)

(event `StopAltFire`)

(fn `AttachToOwner`
  (`SceneComponent.K2_AttachToComponent` (`self.WeaponMesh`) (`/Game/Prototype/Characters/BP_PlayerCharacter.FirstPersonMesh` (`self.WeaponOwner`)) (`self.HandsAttachSocket`) "SnapToTarget" "SnapToTarget" "SnapToTarget" true))

(fn `DetachFromOwner`)

(fn `FireInstantHit`)

(fn `FireProjectile`)

(fn `GiveTo`
  (params (Owner :type "/Game/Prototype/Characters/BP_PlayerCharacter Object Reference"))
  (set `self.WeaponOwner` Owner)
  (`self.SetOwner` Owner)
  (set `self.Instigator` Owner))

(fn `Remove`
  (set `self.WeaponOwner` null)
  (`self.SetOwner` null)
  (set `self.Instigator` null))

(fn `UserConstructionScript`)