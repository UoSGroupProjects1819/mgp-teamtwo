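; BP_Zombie is a prototype AI zombie character that drops into a ragdoll when it takes damage.
; Any damage above zero triggers this, with no health tracking in the graph.
; The damage event stops movement, switches the mesh to physics simulation with collision, and disables capsule collision.
; The construction script only calls its parent.
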(event `self.ReceiveAnyDamage`
  (params (Damage :type "Float (single-precision)") (DamageType :type "DamageType Object Reference") (InstigatedBy :type "Controller Object Reference") (DamageCauser :type "Actor Object Reference"))
  (bind _mesh (`self.Mesh`))
  (if (> Damage 0.0)
    (`MovementComponent.StopMovementImmediately` (`self.CharacterMovement`))
    (`PrimitiveComponent.WakeAllRigidBodies` (`self.Mesh`))
    (`PrimitiveComponent.SetSimulatePhysics` _mesh true)
    (`PrimitiveComponent.SetCollisionEnabled` _mesh "QueryAndPhysics")
    (`PrimitiveComponent.SetCollisionEnabled` (`self.CapsuleComponent`) "NoCollision")))

(fn `UserConstructionScript`
  (`parent.UserConstructionScript`))