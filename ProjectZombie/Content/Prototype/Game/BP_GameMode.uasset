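; Game mode that populates the level with AI zombies if the game begins at night.
; On BeginPlay it asks the first BP_Sky_Sphere actor whether it is night, with no later re-check.
; If so, it spawns a BP_Zombie running Zombie_BehaviorTree at each PlayerStart tagged "Zombie", reusing those actors as enemy spawn points.
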(event `self.ReceiveBeginPlay`
  (bind _outactors (`GameplayStatics.GetAllActorsOfClass` "/Engine/EngineSky/BP_Sky_Sphere.BP_Sky_Sphere_C"))
  (if (`/Engine/EngineSky/BP_Sky_Sphere.GetIsNight` (`|GetArrayItem` _outactors))
    (bind _outactors_2 (`GameplayStatics.GetAllActorsOfClass` "/Script/Engine.PlayerStart"))
    (for _array_element _outactors_2
      (if (== (`PlayerStart.PlayerStartTag` _array_element) "Zombie")
        (`AIBlueprintHelperLibrary.SpawnAIFromClass` "/Game/Prototype/AI/BP_Zombie.BP_Zombie_C" "/Game/Prototype/AI/Zombie_BehaviorTree.Zombie_BehaviorTree" (`self.K2_GetActorLocation` _array_element) (`self.K2_GetActorRotation` _array_element))))))

(fn `UserConstructionScript`)