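; Behavior tree service that updates a zombie's blackboard to choose between a heard distraction and the player as target.
; On activation it writes the waypoint to the patrol key.
; Each tick, while sound age is under five seconds, it queries AI Perception hearing.
; A heard actor (last in the list) becomes the distraction and clears the player key; otherwise the distraction clears and the player pawn is set.
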(event `self.ReceiveActivationAI`
  (params (OwnerController :type "AIController Object Reference") (ControlledPawn :type "Pawn Object Reference"))
  ;[0 0 0] Called on AI start
  (`BTFunctionLibrary.SetBlackboardValueAsObject` (`self.PatrolKey`) "/Game/Blueprints/AI/Waypoint.Waypoint"))

(event `self.ReceiveTickAI`
  (params (OwnerController :type "AIController Object Reference") (ControlledPawn :type "Pawn Object Reference") (DeltaSeconds :type "Float (single-precision)"))
  ;[0 0 0] Update zombie AI state and blackbaord values every frame
  (bind _aszombie (cast `/Game/Blueprints/AI/Zombie` ControlledPawn))
  (if (< (`BlackboardComponent.GetValueAsFloat` (`AIBlueprintHelperLibrary.GetBlackboard` _aszombie) (`self.SoundAgeKey`)) 5.0)
    (bind _outactors (`AIPerceptionComponent.GetPerceivedActors` (`/Game/Blueprints/AI/Zombie.AIPerception` _aszombie) "/Script/AIModule.AISense_Hearing"))
    (if (> (`KismetArrayLibrary.Array_Length` _outactors) 0)
      (for _array_element _outactors
        _)
      (`BTFunctionLibrary.SetBlackboardValueAsObject` (`self.DistractionKey`) _array_element)
      (`BTFunctionLibrary.SetBlackboardValueAsObject` (`self.PlayerKey`))
      (else
        (for _array_element_2 _outactors
          (`KismetArrayLibrary.Array_RemoveItem` _outactors _array_element_2))
        (`BTFunctionLibrary.SetBlackboardValueAsObject` (`self.DistractionKey`))
        (`BTFunctionLibrary.SetBlackboardValueAsObject` (`self.PlayerKey`) (`self.PlayerPawn`))))))