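; Behavior tree service that switches a PZZombie between chasing heard sounds and targeting the player.
; Each AI tick, while the blackboard SoundAge is under a fixed threshold, it queries the perception component for hearing-perceived actors.
; If any exist, the last becomes SoundTarget and PlayerTarget is cleared.
; Otherwise SoundTarget is cleared and PlayerTarget becomes the player pawn.
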(event `self.ReceiveTickAI`
  (params (OwnerController :type "AIController Object Reference") (ControlledPawn :type "Pawn Object Reference") (DeltaSeconds :type "Float (single-precision)"))
  (bind _aspzzombie (cast `PZZombie` ControlledPawn))
  (if (< (`BlackboardComponent.GetValueAsFloat` (`AIBlueprintHelperLibrary.GetBlackboard` _aspzzombie) (`self.SoundAge`)) 5.0)
    (bind _outactors (`AIPerceptionComponent.GetPerceivedActors` (`Actor.GetComponentByClass` _aspzzombie "/Script/AIModule.AIPerceptionComponent") "/Script/AIModule.AISense_Hearing"))
    (if (> (`KismetArrayLibrary.Array_Length` _outactors) 0)
      (for _array_element _outactors
        _)
      (`BTFunctionLibrary.SetBlackboardValueAsObject` (`self.SoundTarget`) _array_element)
      (`BTFunctionLibrary.SetBlackboardValueAsObject` (`self.PlayerTarget`))
      (else
        (for _array_element_2 _outactors
          (`KismetArrayLibrary.Array_RemoveItem` _outactors _array_element_2))
        (`BTFunctionLibrary.SetBlackboardValueAsObject` (`self.SoundTarget`))
        (`BTFunctionLibrary.SetBlackboardValueAsObject` (`self.PlayerTarget`) "/Game/Blueprints/Pawns/PlayerPawn.PlayerPawn")))))