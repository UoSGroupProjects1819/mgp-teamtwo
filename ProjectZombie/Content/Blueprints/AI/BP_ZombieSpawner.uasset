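; BP_ZombieSpawner periodically spawns AI zombies for a survival game mode.
; A looping five-second timer calls Spawn, which checks MaxZombies against NumZombie and finds a "Zombie" player start through GameMode_Survival.
; The Zombies loop has an empty body, so one spawn follows it using the final array element and Zombie_BT.
; NumZombie is then set to a constant one rather than incremented.
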(event `self.ReceiveBeginPlay`
  (`KismetSystemLibrary.K2_SetTimer` null "Spawn" 5.0 true))

(event `Spawn`
  (if (>= (`self.MaxZombies`) (`self.NumZombie`))
    (bind _asgame_mode_survival (cast `/Game/Blueprints/Game/GameMode_Survival` (`GameplayStatics.GetGameMode`)))
    (for _array_element (`self.Zombies`)
      _)
    (`AIBlueprintHelperLibrary.SpawnAIFromClass` _array_element "/Game/Blueprints/AI/Zombie_BT.Zombie_BT" (`self.K2_GetActorLocation` (`GameModeBase.K2_FindPlayerStart` _asgame_mode_survival (`AIBlueprintHelperLibrary.GetAIController` null) "Zombie")))
    (set `self.NumZombie` (+ 0 1))))

(fn `UserConstructionScript`)