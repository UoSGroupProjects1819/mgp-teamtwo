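; Sky manager actor meant to animate a day cycle by rotating a referenced Sun actor on Tick.
; It updates only when LastTimeDay exactly equals the game state's time since creation, then stores its own creation time.
; Elapsed time plus a predicted increment drives the Sun's roll with an offset, at fixed pitch.
; As written, the day-length divisor evaluates to zero, and the construction script is empty.
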(event `self.ReceiveTick`
  (params (DeltaSeconds :type "Float (single-precision)"))
  (if (`KismetSystemLibrary.IsValid` (`self.Sun`))
    (if (== (`self.LastTimeDay`) (`self.GetGameTimeSinceCreation` (`GameplayStatics.GetGameState`)))
      (set `self.TimeSinceLastDay` (+ DeltaSeconds 1.0))
      (set `self.PredictedMovement` (* (`self.TimeofDayIncrement`) (`self.LastTimeDay`)))
      (set `self.DayMinutes` (* 60.0 0.0))
      (set `self.PitchRotation` (* 360.0 (/ (+ (`self.GetGameTimeSinceCreation`) (`self.PredictedMovement`)) (`self.DayMinutes`))))
      (`self.K2_SetActorRelativeRotation` (`self.Sun`) (`KismetMathLibrary.MakeRotator` (+ (`self.PitchRotation`) (`self.PitchOffset`)) 45.0) false false)
      (set `self.LastTimeDay` (`self.GetGameTimeSinceCreation`))
      (else
        (set `self.TimeSinceLastDay` 0.0)))))

(fn `UserConstructionScript`)