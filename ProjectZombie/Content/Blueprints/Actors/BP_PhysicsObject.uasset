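; BP_PhysicsObject is a physics-object actor that hurts zombies its Box component hits.
; The hit event casts the other actor to BP_Zombie and applies its Damage and DamageType, crediting the first player controller as instigator.
; On a blocking hit, it also breaks the zombie mesh's constraint at the hit bone with zero impulse, detaching that body part.
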(event `self.Box.OnComponentHit`
  (params (HitComponent :type "PrimitiveComponent Object Reference") (OtherActor :type "Actor Object Reference") (OtherComp :type "PrimitiveComponent Object Reference") (NormalImpulse :type "Vector Structure") (Hit :type "HitResult Structure (by ref)"))
  (bind (_bblockinghit _binitialoverlap _time _distance _location _impactpoint _normal _impactnormal _physmat _hitactor _hitcomponent _hitbonename) (`GameplayStatics.BreakHitResult` Hit))
  (`/Engine/EditorBlueprintResources/StandardMacros.IsValid` OtherActor
    (:`Is Valid`
      (bind _asbp_zombie (cast `/Game/Blueprints/AI/BP_Zombie` OtherActor))
      (`GameplayStatics.ApplyDamage` _asbp_zombie (`self.Damage`) (`GameplayStatics.GetPlayerController` 0) self (`self.DamageType`))
      (if _bblockinghit
        (bind _asbp_zombie_2 (cast `/Game/Blueprints/AI/BP_Zombie` _hitactor))
        (`SkeletalMeshComponent.BreakConstraint` (`Character.Mesh` _asbp_zombie_2) (0.0 0.0 0.0) _location _hitbonename)))))

(fn `UserConstructionScript`)